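; BP_ShipManager is an interactable actor that pairs a panel button with a ship manager panel, each held as a child actor.
; Its construction script casts both child actors and adds the panel to the button's linked interactables.
; It then moves the panel's ship spawn component to the manager's ShipSpawnLocation.
; The event graph has no active logic, so all wiring happens at construction.
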(fn `UserConstructionScript`
  ;[1 1 1] Create the link between the ship manager's button and panel
  (bind _asbp_panel_button (cast `/Game/Interactables/C/BP_PanelButton` (`ChildActorComponent.ChildActor` (`self.ButtonChildActor`))))
  (bind _asbp_ship_manager_panel (cast `/Game/Interactables/C/BP_ShipManagerPanel` (`ChildActorComponent.ChildActor` (`self.PanelChildActor`))))
  (`KismetArrayLibrary.Array_Add` (`PanelButton.LinkedInteractables` _asbp_panel_button) _asbp_ship_manager_panel)
  (`SceneComponent.K2_SetWorldLocation` (`ShipManagerPanel.ShipSpawnComponent` _asbp_ship_manager_panel) (`self.ShipSpawnLocation`) false false))